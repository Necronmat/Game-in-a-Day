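; BP_GameInADayGameModeBase is the game mode for a turn-based piece game, relaying game events to the UI.
; GameOver creates the WBP_GameOver widget, pauses the game, switches input to UI only and passes in the winner.
; DisplayHover, DisplayPlayersTurn and DisplaySpace look up top-level WBP_GameUI widgets on each call and forward the selected piece, current player or space coordinates.
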(event EventTick
  (params (DeltaSeconds :type Float%20%28single-precision%29)))

(event EventGameOver
  (params (winner :type Integer))
  (bind _returnvalue (UserInterface|CreateWidget "/Game/UI/WBP_GameOver.WBP_GameOver_C"))
  (UserInterface|Viewport|AddtoViewport _returnvalue 0)
  (Game|SetGamePaused true)
  (Input|SetInputModeUIOnly (Game|GetPlayerController 0) _returnvalue "DoNotLock")
  (Default|WinnersText _returnvalue winner))

(event EventDisplayHover
  (params (player :type Integer) (piece :type Integer))
  (bind _foundwidgets (Widget|GetAllWidgetsOfClass "/Game/UI/WBP_GameUI.WBP_GameUI_C" true))
  (Default|SelectedPiece _foundwidgets player piece))

(event EventDisplayPlayersTurn
  (params (player :type Integer))
  (bind _foundwidgets (Widget|GetAllWidgetsOfClass "/Game/UI/WBP_GameUI.WBP_GameUI_C" true))
  (Default|DisplayPlayerTurn _foundwidgets player))

(event EventDisplaySpace
  (params (x :type Integer) (y :type Integer))
  (bind _foundwidgets (Widget|GetAllWidgetsOfClass "/Game/UI/WBP_GameUI.WBP_GameUI_C" true))
  (Default|DisplaySpace _foundwidgets x y))

(fn ConstructionScript)